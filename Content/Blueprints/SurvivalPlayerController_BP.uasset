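; Player controller Blueprint for the survival game that toggles the inventory screen on the OpenInventory input.
; The inventory widget is created on first use and cached for later presses.
; Opening adds it to the viewport, shows the mouse cursor and sets Game and UI input mode focused on the widget.
; Closing is delegated to the widget's own CloseInventory function.
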(event `InputAction|OpenInventory`
  (params (Key :type "Key Structure"))
  (bind _inventorywidget (`self.InventoryWidget`))
  (:`Pressed`
    (`/Engine/EditorBlueprintResources/StandardMacros.IsValid` (`self.InventoryWidget`)
      (:`Is Valid`
        (if (`Widget.IsInViewport` _inventorywidget)
          (`/Game/UserInterface/Widgets/WBP_Inventory.CloseInventory` _inventorywidget)
          (else
            (`UserWidget.AddToViewport` (stale _output_get) 0 :!label _label)
            (set `self.bShowMouseCursor` true)
            (`WidgetBlueprintLibrary.SetInputMode_GameAndUIEx` self (`self.InventoryWidget`)))))
      (:`Is Not Valid`
        (bind _returnvalue (`|CreateWidget` "/Game/UserInterface/Widgets/WBP_Inventory.WBP_Inventory_C" self))
        (bind _output_get (set `self.InventoryWidget` _returnvalue))
        (goto _label)))))

(fn `UserConstructionScript`)